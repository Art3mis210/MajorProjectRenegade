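; Quest NPC that roams spline paths and holds voiced Narrative dialogue with the player.
; In Walking behaviour it follows the nearest NPCPath point by point with randomized destinations, periodically re-picking path and direction at random.
; A box overlap begins the quest dialogue, voicing NPC lines and forwarding player lines to the character.
; Speech uses runtime AzSpeech text-to-speech with random talk poses, then advances any current group's dialogue.
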(event `Roam`
  (bind _spline (`/Game/Sachit/Blueprints/NPCPath/NPCPath.Spline` (`self.npcPath`)))
  (bind _returnvalue (`SplineComponent.GetNumberOfSplinePoints` _spline))
  ;[1 1 1] Roam
  (bind _randomlocation (`NavigationSystemV1.K2_GetRandomLocationInNavigableRadius` (`SplineComponent.GetLocationAtSplinePoint` _spline (`self.SplinePointIndex`) "World") 100.0 null null))
  (`|AIMoveTo` self _randomlocation null 100.0
    (:`OnSuccess`
      (if (`self.WalkDirectionForward`)
        (set `self.SplinePointIndex` (mod (+ (`self.SplinePointIndex`) 1) _returnvalue))
        (else
          (set `self.SplinePointIndex` (mod (- (`self.SplinePointIndex`) 1) _returnvalue))))
      (`self.Roam`)
      (bind _output_get (set `self.PathChangeTimer` (- (`self.PathChangeTimer`) 1.0)))
      (if (<= _output_get 0.0)
        (if (== (`KismetMathLibrary.RandomInteger` 3) 2)
          (`self.FindNearbySplineForWalking`)
          (set `self.PathChangeTimer` (`KismetMathLibrary.Conv_IntToDouble` (+ (`KismetMathLibrary.RandomInteger` 50) 10))))))))

(event `FindNearbySplineForWalking`
  (bind _returnvalue (`self.K2_GetActorLocation`))
  (bind _spline (`/Game/Sachit/Blueprints/NPCPath/NPCPath.Spline` (`self.npcPath`)))
  ;[1 1 1] Find Nearest Path
  (bind _outactors (`GameplayStatics.GetAllActorsOfClass` "/Game/Sachit/Blueprints/NPCPath/NPCPath.NPCPath_C"))
  (bind _asnpcpath (cast `/Game/Sachit/Blueprints/NPCPath/NPCPath` (`.ReturnValue` (`GameplayStatics.FindNearestActor` (`self.K2_GetActorLocation`) _outactors))))
  (set `self.npcPath` _asnpcpath)
  (set `self.WalkDirectionForward` (`KismetMathLibrary.RandomBool`))
  (set `self.SplinePointIndex` 0)
  (for _index (range 1 (+ (- (`SplineComponent.GetNumberOfSplinePoints` _spline) 0) 1))
    (if (< (`KismetMathLibrary.Vector_Distance` (`SplineComponent.GetLocationAtSplinePoint` _spline _index "World") _returnvalue) (`KismetMathLibrary.Vector_Distance` _returnvalue (`SplineComponent.GetLocationAtSplinePoint` _spline (`self.SplinePointIndex`) "World")))
      (set `self.SplinePointIndex` _index))))

(event `self.ReceiveBeginPlay`
  (`self.UpdateBehaviour` (`self.Behaviour`))
  (bind _askid_abp (cast `/Game/Sachit/Characters/MainPlayer/Kid/Blueprints/KidABP` (`SkeletalMeshComponent.GetAnimInstance` (`self.Mesh`))))
  (set `self.AnimationBlueprint` _askid_abp)
  (bind _returnvalue (`|CreateWidget` "/Narrative/NarrativeUI/Widgets/BP_NarrativeDefaultUI.BP_NarrativeDefaultUI_C" null (`self.Narrative`)))
  (`UserWidget.AddToViewport` _returnvalue 0))

(event `Speak`
  (params (Dialogue :type String))
  (bind _animationblueprint (`self.AnimationBlueprint`))
  (bind _currentgroup (`self.CurrentGroup`))
  ;[0 0 0] Speak
  (bind (_asynctaskproxy _generatedsound) (`TextToSoundWaveAsync.TextToSoundWave_CustomOptions` (make `AzSpeechSubscriptionOptions` "2df52676806c4dc1b115d0f78e7b77bd") (make `AzSpeechSynthesisOptions` "en-US" (`KismetStringLibrary.Conv_StringToName` (`|GetEnumeratorNameAsString` (`self.VoiceType`)))) Dialogue)
    (:`SynthesisCompleted`
      (`GameplayStatics.SpawnSoundAttached` _generatedsound (`self.Mesh`) "None" (0.0 0.0 0.0) (struct) "KeepRelativeOffset" true 1.0 1.0 0.0 "/Game/Sachit/Voice/VoiceAttenuation.VoiceAttenuation" null)
      (set `/Game/Sachit/Characters/MainPlayer/Kid/Blueprints/KidABP.SpeakPose` (`KismetMathLibrary.Conv_IntToDouble` (`KismetMathLibrary.RandomInteger` 4)) _animationblueprint)
      (set `/Game/Sachit/Characters/MainPlayer/Kid/Blueprints/KidABP.Speak` true _animationblueprint)
      (`KismetSystemLibrary.Delay` (`SoundBase.Duration` _generatedsound))
      (`/Engine/EditorBlueprintResources/StandardMacros.IsValid` _currentgroup
        (:`Is Valid`
          (`/Game/GroupDialogue.PlayDialogue` _currentgroup))
        (:`Is Not Valid`
          _))
      (set `/Game/Sachit/Characters/MainPlayer/Kid/Blueprints/KidABP.Speak` false _animationblueprint))))

(event `self.Box.OnComponentBeginOverlap`
  (params (OverlappedComponent :type "PrimitiveComponent Object Reference") (OtherActor :type "Actor Object Reference") (OtherComp :type "PrimitiveComponent Object Reference") (OtherBodyIndex :type Integer) (bFromSweep :type Boolean) (SweepResult :type "HitResult Structure (by ref)"))
  ;[0 0 0] Start Dialogue
  (bind _asbp_third_person_character (cast `/Game/ThirdPerson/Blueprints/BP_ThirdPersonCharacter` OtherActor))
  (set `self.Player` _asbp_third_person_character)
  (`NarrativeComponent.BeginDialogue` (`self.Narrative`) (`self.QuestDialogue`) null "None"))

(event `self.Narrative.OnNPCDialogueLineStarted`
  (params (Dialogue :type "Dialogue Object Reference") (Node :type "DialogueNode_NPC Object Reference") (DialogueLine :type "DialogueLine Structure (by ref)") (Speaker :type "SpeakerInfo Structure (by ref)"))
  (`self.Speak` (`KismetTextLibrary.Conv_TextToString` (`DialogueNode.Text` Node))))

(event `self.Narrative.OnPlayerDialogueLineStarted`
  (params (Dialogue :type "Dialogue Object Reference") (Node :type "DialogueNode_Player Object Reference") (DialogueLine :type "DialogueLine Structure (by ref)"))
  (`/Game/ThirdPerson/Blueprints/BP_ThirdPersonCharacter.Speak` (`self.Player`) (`KismetTextLibrary.Conv_TextToString` (`DialogueNode.Text` Node))))

(fn `RemoveFromGroup`
  (set `self.CurrentGroup` null))

(fn `SetCurrentGroup`
  (params (Group :type "/Game/GroupDialogue Object Reference"))
  (set `self.CurrentGroup` Group))

(fn `UpdateBehaviour`
  (params (`New Behaviour` :type "/Game/Sachit/Blueprints/NPC/NPC_Behaviour Enum" :default "NewEnumerator1"))
  (bind _output_get (set `self.Behaviour` `New Behaviour`))
  (switch `/Game/Sachit/Blueprints/NPC/NPC_Behaviour` _output_get
    (:`NewEnumerator2`
      (`self.FindNearbySplineForWalking`)
      (`self.Roam`))))

(fn `UserConstructionScript`)