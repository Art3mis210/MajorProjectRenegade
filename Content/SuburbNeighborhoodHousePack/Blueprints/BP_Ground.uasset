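; BP_Ground is a ground piece in the Suburb Neighborhood House Pack whose mesh is chosen from a list of variants.
; The construction script indexes GroundMeshes with the Ground value and assigns the result to the GroundMesh component.
; RevertDefaultMaterials acts as a one-shot toggle that copies the chosen mesh's default materials back onto each component slot, then clears itself.
; The event graph contains no active logic.
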(fn `UserConstructionScript`
  (locals (`Number Of Materials` :type Integer) (New_mesh :type "StaticMesh Object Reference"))
  (bind _ground_mesh (`self.Ground_mesh`))
  (bind _output (`|GetArrayItem` (`self.Ground Meshes`) (`KismetMathLibrary.Conv_ByteToInt` (`self.Ground`))))
  (`StaticMeshComponent.SetStaticMesh` (`self.Ground_mesh`) _output)
  (set `local.New_mesh` _output)
  (if (`self.Revert Default Materials`)
    (bind _output_get (set `local.Number Of Materials` (`PrimitiveComponent.GetNumMaterials` _ground_mesh)))
    (for _index (range (+ _output_get 1))
      (`PrimitiveComponent.SetMaterial` _ground_mesh _index (`StaticMesh.GetMaterial` (`local.New_mesh`) _index)))
    (set `self.Revert Default Materials` false)))