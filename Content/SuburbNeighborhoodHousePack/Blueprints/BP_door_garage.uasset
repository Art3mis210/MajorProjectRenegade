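; Garage door actor that opens and closes on an OpenClose event unless it is locked.
; A timeline lerps the door mesh between closed and open transforms, reversing to close and marking it closed only when backward playback finishes.
; The construction script picks the door mesh from the DoorsGarage selection, with a matching 3x or 5x frame mesh.
; A one-shot RevertDefaultMaterials toggle restores the selected mesh's default materials.
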(event `OpenClose`
  (if (`self.Locked`)
    _
    (elif (`self.DoorClosed`)
      (set `self.DoorClosed` false)
      (bind (_direction _dooranimation) (`Timeline|DoorAnim` :!label _label)
        (:`Update`
          (`SceneComponent.K2_SetRelativeTransform` (`self.Door_garage_mesh`) (`KismetMathLibrary.TLerp` (`self.Door_closed_transform`) (`self.Door_open_transform`) _dooranimation) false false))
        (:`Finished`
          (switch `ETimelineDirection` _direction
            (:`Backward`
              (set `self.DoorClosed` true)))))
      (else
        (goto _label :!via `Reverse`)))))

(fn `UserConstructionScript`
  (locals (New_mesh :type "StaticMesh Object Reference") (`Number Of Materials` :type Integer))
  (bind _door_garage_frames (`self.Door_garage_frames`))
  (bind _door_garage_mesh (`self.Door_garage_mesh`))
  (bind _returnvalue (`PrimitiveComponent.GetNumMaterials` _door_garage_mesh))
  (bind _returnvalue_2 (`KismetMathLibrary.Conv_ByteToInt` (`self.Doors_garage`)))
  (bind _output (`|GetArrayItem` (`self.Door Meshes`) _returnvalue_2))
  (`StaticMeshComponent.SetStaticMesh` (`self.Door_garage_mesh`) _output)
  (set `local.New_mesh` _output)
  (`/Engine/EditorBlueprintResources/StandardMacros.CompareInt` _returnvalue_2 1
    (:`>`
      (`StaticMeshComponent.SetStaticMesh` _door_garage_frames "/Game/SuburbNeighborhoodHousePack/Meshes/Meshes_replacedwithBlueprints/SM_Door_garage_frames_5x.SM_Door_garage_frames_5x"))
    (:`==`
      (`StaticMeshComponent.SetStaticMesh` _door_garage_frames "/Game/SuburbNeighborhoodHousePack/Meshes/Meshes_replacedwithBlueprints/SM_Door_garage_frames_3x.SM_Door_garage_frames_3x" :!label _label))
    (:`<`
      (goto _label)))
  (if (`self.Revert Default Materials`)
    (set `local.Number Of Materials` _returnvalue)
    (for _index (range (+ _returnvalue 1))
      (`PrimitiveComponent.SetMaterial` _door_garage_mesh _index (`StaticMesh.GetMaterial` (`local.New_mesh`) _index)))
    (set `self.Revert Default Materials` false)))