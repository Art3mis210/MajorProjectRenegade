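; BP_Porch is a porch building piece from the suburban house pack, with a selectable mesh variant.
; The construction script uses the Porch value to index the PorchMeshes array and assigns that static mesh to the PorchMesh component.
; RevertDefaultMaterials acts as a one-shot toggle that copies the selected mesh's default materials back onto the component, then resets itself.
; The event graph holds only disabled placeholder events, so there is no runtime logic.
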(fn `UserConstructionScript`
  (locals (`Number Of Materials` :type Integer) (New_mesh :type "StaticMesh Object Reference"))
  (bind _porch_mesh (`self.Porch_mesh`))
  (bind _output (`|GetArrayItem` (`self.Porch Meshes`) (`KismetMathLibrary.Conv_ByteToInt` (`self.Porch`))))
  (`StaticMeshComponent.SetStaticMesh` (`self.Porch_mesh`) _output)
  (set `local.New_mesh` _output)
  (if (`self.Revert Default Materials`)
    (bind _output_get (set `local.Number Of Materials` (`PrimitiveComponent.GetNumMaterials` _porch_mesh)))
    (for _index (range (+ _output_get 1))
      (`PrimitiveComponent.SetMaterial` _porch_mesh _index (`StaticMesh.GetMaterial` (`local.New_mesh`) _index)))
    (set `self.Revert Default Materials` false)))