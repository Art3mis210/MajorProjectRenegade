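; Traffic light actor that cycles its signal and halts or releases AI_Car vehicles entering its box.
; A looping BeginPlay timer uses a FlipFlop to alternate green and red, always passing through yellow, with red held longer.
; Each switch sets TrafficLightState, true only for green, and shows the matching lamp mesh.
; Box overlap stops the car on non-green, rechecking via a shared Retriggerable Delay until green calls Driving.
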(event `self.ReceiveBeginPlay`
  (`KismetSystemLibrary.Delay` 10.0 :!label _label)
  (`self.SwitchToYellow`)
  (`KismetSystemLibrary.Delay` 2.0)
  (`/Engine/EditorBlueprintResources/StandardMacros.FlipFlop`
    (:`A`
      (`self.SwitchToGreen`)
      (goto _label))
    (:`B`
      (`self.SwitchToRed`)
      (`KismetSystemLibrary.Delay` 10.0)
      (goto _label))))

(event `self.Box.OnComponentBeginOverlap`
  (params (OverlappedComponent :type "PrimitiveComponent Object Reference") (OtherActor :type "Actor Object Reference") (OtherComp :type "PrimitiveComponent Object Reference") (OtherBodyIndex :type Integer) (bFromSweep :type Boolean) (SweepResult :type "HitResult Structure (by ref)"))
  (bind _asai_car (cast `/Game/VehicleTemplate/Blueprints/SportsCar/AI_Car` OtherActor))
  (if (`self.TrafficLightState`) :!label _label_2
    (`/Game/VehicleTemplate/Blueprints/SportsCar/AI_Car.Driving` _asai_car)
    (else
      (`/Game/VehicleTemplate/Blueprints/SportsCar/AI_Car.Stop` _asai_car)
      (`KismetSystemLibrary.RetriggerableDelay` 1.0)
      (goto _label_2))))

(fn `SwitchToGreen`
  (set `self.TrafficLightState` true)
  (`|ExecutionSequence`
    (:`then_0`
      (`SceneComponent.SetHiddenInGame` (`self.Traffic_light_animated_Traffic_Light_green`) false false))
    (:`then_1`
      (`SceneComponent.SetHiddenInGame` (`self.Traffic_light_animated_Traffic_Light_orange`) true false)
      (`SceneComponent.SetHiddenInGame` (`self.Traffic_light_animated_Traffic_Light_red`) true false))))

(fn `SwitchToRed`
  (set `self.TrafficLightState` false)
  (`|ExecutionSequence`
    (:`then_0`
      (`SceneComponent.SetHiddenInGame` (`self.Traffic_light_animated_Traffic_Light_red`) false false))
    (:`then_1`
      (`SceneComponent.SetHiddenInGame` (`self.Traffic_light_animated_Traffic_Light_green`) true false)
      (`SceneComponent.SetHiddenInGame` (`self.Traffic_light_animated_Traffic_Light_orange`) true false))))

(fn `SwitchToYellow`
  (set `self.TrafficLightState` false)
  (`|ExecutionSequence`
    (:`then_0`
      (`SceneComponent.SetHiddenInGame` (`self.Traffic_light_animated_Traffic_Light_orange`) false false))
    (:`then_1`
      (`SceneComponent.SetHiddenInGame` (`self.Traffic_light_animated_Traffic_Light_green`) true false)
      (`SceneComponent.SetHiddenInGame` (`self.Traffic_light_animated_Traffic_Light_red`) true false))))

(fn `UserConstructionScript`)