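; BP_Interior_Walls is a modular interior wall actor from the suburban house pack that lets the wall piece be chosen per instance.
; The construction script uses the WallsInterior selection to pick a mesh from WallMeshes and assigns it to WallMesh.
; RevertDefaultMaterials acts as a one-shot toggle that copies the selected mesh's default materials back onto each slot, then clears itself.
; It has no active runtime logic.
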(fn `UserConstructionScript`
  (locals (`Number Of Materials` :type Integer) (New_mesh :type "StaticMesh Object Reference"))
  (bind _wall_mesh (`self.Wall_mesh`))
  (bind _output (`|GetArrayItem` (`self.Wall Meshes`) (`KismetMathLibrary.Conv_ByteToInt` (`self.Walls Interior`))))
  (`StaticMeshComponent.SetStaticMesh` (`self.Wall_mesh`) _output)
  (set `local.New_mesh` _output)
  (if (`self.Revert Default Materials`)
    (bind _output_get (set `local.Number Of Materials` (`PrimitiveComponent.GetNumMaterials` _wall_mesh)))
    (for _index (range (+ _output_get 1))
      (`PrimitiveComponent.SetMaterial` _wall_mesh _index (`StaticMesh.GetMaterial` (`local.New_mesh`) _index)))
    (set `self.Revert Default Materials` false)))