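; Male_NPC is an NPC Blueprint that patrols endlessly along a spline path.
; On BeginPlay it calls Roam, which uses AIMoveTo toward the current spline point of its Path reference in world space.
; Each successful move advances the point index with a modulo wrap and calls Roam again, looping the route.
; Failed moves are not handled, so the patrol stops if one fails.
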(event `Roam`
  (bind _spline (`/Game/Sachit/Blueprints/NPCPath/NPCPath.Spline` (`self.Path`)))
  (`|AIMoveTo` self (`SplineComponent.GetLocationAtSplinePoint` _spline (`self.SplinePointIndex`) "World") null
    (:`OnSuccess`
      (set `self.SplinePointIndex` (mod (+ (`self.SplinePointIndex`) 1) (`SplineComponent.GetNumberOfSplinePoints` _spline)))
      (`self.Roam`))))

(event `self.ReceiveBeginPlay`
  (`self.Roam`))

(fn `UserConstructionScript`)