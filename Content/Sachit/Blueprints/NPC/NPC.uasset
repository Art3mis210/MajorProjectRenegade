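; High school NPC character that walks spline paths, follows or flees the player, and holds AI-driven spoken conversations.
; A behaviour state starts roaming along the nearest NPCPath (occasionally re-picking it), following, or running away.
; Player messages go with name, personality and previous response to a chat model, whose JSON returns a line and an action, such as following.
; AzSpeech voices lines, drives the talk animation and advances group dialogue.
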(event Custom|Roam
  (bind _npcpath (Variables|Movement|GetnpcPath))
  (bind _spline (Variables|/Game/Sachit/Blueprints/NPCPath/NPCPath.NPCPath_C|GetSpline _npcpath))
  (bind _returnvalue (Spline|GetNumberOfSplinePoints _spline))
  ;[1 1 1] Roam
  (if (Utilities|Enum|Equal(Enum) (Variables|Movement|GetBehaviour) "NewEnumerator2")
    (bind _randomlocation (Class|NavigationSystemV1|GetRandomLocationinNavigableRadius (Spline|GetLocationatSplinePoint _spline (Variables|Movement|GetSplinePointIndex) "World") 1e+02 0 0))
    (AI|AIMoveTo self _randomlocation 0 1e+02 false
      (:OnSuccess
        (if (Utilities|Enum|Equal(Enum) (Variables|Movement|GetBehaviour) "NewEnumerator2")
          (if (Variables|Movement|GetWalkDirectionForward)
            (Variables|Movement|SetSplinePointIndex (Math|Integer|%(Integer) (+ (Variables|Movement|GetSplinePointIndex) 1) _returnvalue))
            (else
              (Variables|Movement|SetSplinePointIndex (Math|Integer|%(Integer) (- (Variables|Movement|GetSplinePointIndex) 1) _returnvalue))))
          (CallFunction|Roam)
          (bind _output_get (Variables|Movement|SetPathChangeTimer (- (Variables|Movement|GetPathChangeTimer) 1.0)))
          (if (<= _output_get 0.0)
            (if (== (Math|Random|RandomInteger 3) 2)
              (CallFunction|FindNearbySplineforWalking)
              (Variables|Movement|SetPathChangeTimer (Math|Conversions|ToFloat(Integer) (+ (Math|Random|RandomInteger 50) 10))))))))))

(event Custom|FindNearbySplineForWalking
  (bind _returnvalue (Transformation|GetActorLocation))
  ;[1 1 1] Find Nearest Path
  (if (Utilities|Enum|Equal(Enum) (Variables|Movement|GetBehaviour) "NewEnumerator2")
    (bind _outactors (Actor|GetAllActorsOfClass "/Game/Sachit/Blueprints/NPCPath/NPCPath.NPCPath_C"))
    (bind _asnpcpath (Utilities|Casting|CastToNPCPath (.ReturnValue (Actor|FindNearestActor (Transformation|GetActorLocation) _outactors))))
    (Variables|Movement|SetnpcPath _asnpcpath)
    (Variables|Movement|SetWalkDirectionForward (Math|Random|RandomBool))
    (Variables|Movement|SetSplinePointIndex 0)
    (for _index (range 1 (- (Spline|GetNumberOfSplinePoints (Variables|/Game/Sachit/Blueprints/NPCPath/NPCPath.NPCPath_C|GetSpline (Variables|Movement|GetnpcPath))) 0))
      (if (< (Math|Vector|Distance(Vector) (Spline|GetLocationatSplinePoint (Variables|/Game/Sachit/Blueprints/NPCPath/NPCPath.NPCPath_C|GetSpline (Variables|Movement|GetnpcPath)) _index "World") _returnvalue) (Math|Vector|Distance(Vector) _returnvalue (Spline|GetLocationatSplinePoint (Variables|/Game/Sachit/Blueprints/NPCPath/NPCPath.NPCPath_C|GetSpline (Variables|Movement|GetnpcPath)) (Variables|Movement|GetSplinePointIndex) "World")))
        (Variables|Movement|SetSplinePointIndex _index)))))

(event Custom|Speak
  (params (Dialogue :type String))
  (bind _animationblueprint (Variables|Default|GetAnimationBlueprint))
  (bind _currentgroup (Variables|Group|GetCurrentGroup))
  ;[0 0 0] Speak
  (bind _generatedsound (|TexttoSoundWaveCustomOptions (Utilities|Struct|MakeAzSpeechSubscriptionOptions "2df52676806c4dc1b115d0f78e7b77bd" "centralindia" false "https://centralindia.api.cognitive.microsoft.com/sts/v1.0/issuetoken") (Utilities|Struct|MakeAzSpeechSynthesisOptions "en-US" (Utilities|String|StringToName (Utilities|String|EnumtoString (Variables|Dialogue|GetVoiceType)))) Dialogue)
    (:SynthesisCompleted
      (Audio|SpawnSoundAttached _generatedsound (Variables|Character|GetMesh) "None" "0, 0, 0" "0, 0, 0" "KeepRelativeOffset" true 1.0 1.0 0.0 "/Game/Sachit/Voice/VoiceAttenuation.VoiceAttenuation" 0)
      (Variables|/Game/Sachit/Characters/MainPlayer/Kid/Blueprints/KidABP.KidABP_C|SetSpeakPose _animationblueprint (Math|Conversions|ToFloat(Integer) (Math|Random|RandomInteger 4)))
      (Variables|/Game/Sachit/Characters/MainPlayer/Kid/Blueprints/KidABP.KidABP_C|SetSpeak _animationblueprint true)
      (Utilities|FlowControl|Delay (Variables|/Script/Engine.SoundBase|GetDuration _generatedsound))
      (Utilities|IsValid _currentgroup
        (:Is%20Valid
          (Default|PlayDialogue _currentgroup))
        (:Is%20Not%20Valid
          _))
      (Variables|/Game/Sachit/Characters/MainPlayer/Kid/Blueprints/KidABP.KidABP_C|SetSpeak _animationblueprint false)
      (if (Variables|Conversation|GetTalkingToPlayer)
        (Variables|Conversation|SetTalkingToPlayer false)
        (Variables|/Game/ThirdPerson/Blueprints/BP_ThirdPersonCharacter.BP_ThirdPersonCharacter_C|SetTalkingToNPC (Variables|Conversation|GetPlayer) false)
        (if (Utilities|Enum|Equal(Enum) (Variables|Conversation|GetCurrentAction) "follow_Player")
          (CallFunction|UpdateBehaviour "NewEnumerator4"))))))

(event Custom|Talk%20to%20Player
  (params (PlayerMessage :type String) (Player :type BP%20Third%20Person%20Character%20Object%20Reference))
  ;[1 1 1] Talk to Player
  (if (Variables|Conversation|GetPlayerTalkEnabled)
    (CallFunction|UpdateBehaviour "NewEnumerator1")
    (Variables|Conversation|SetPlayer Player)
    (Variables|Conversation|SetTalkingToPlayer true)
    (bind _response (|SendMessageDefaultOptions (Utilities|String|Append "You are an NPC in a high school game, your name is {" (Variables|Conversation|GetName) "}, your personality is {" (Variables|Conversation|GetPersonality) "}  your actions are {" (Variables|Conversation|GetActions) "} The player's name is Chris" "and they say {" PlayerMessage "} Your previous response was {" (Variables|Conversation|GetPreviousResponse) "}.  Return a json with only one message field and one action field to what player has said"))
      (:ProcessCompleted
        (Development|PrintString (.Content (Utilities|Struct|BreakHttpGPTChatMessage (.Message (Utilities|Struct|BreakHttpGPTChatChoice (stale _array_element))))) true true "(R=0.000000,G=0.660000,B=1.000000,A=1.000000)" 1e+02)
        (bind _outjsonobject (Class|JsonBlueprintFunctionLibrary|FromString (.Content (Utilities|Struct|BreakHttpGPTChatMessage (.Message (Utilities|Struct|BreakHttpGPTChatChoice (stale _array_element)))))))
        (bind _outvalue (|GetJsonField _outjsonobject "message"))
        (bind _output_get (Variables|Conversation|SetPreviousResponse _outvalue))
        (CallFunction|Speak _output_get)
        (bind _outvalue_2 (|GetJsonField _outjsonobject "action"))
        (Variables|Conversation|SetCurrentAction _outvalue_2))
      (:RequestFailed
        (Development|PrintString "Failed")))))

(event Custom|Follow%20Player
  (bind _player (Variables|Conversation|GetPlayer))
  (bind _returnvalue (Transformation|GetActorLocation _player))
  ;[1 1 1] Follow Player
  (if (Utilities|Enum|Equal(Enum) (Variables|Movement|GetBehaviour) "NewEnumerator4")
    (if (>= (Math|Vector|Distance(Vector) (Transformation|GetActorLocation) _returnvalue) 5e+02)
      (AI|AIMoveTo self _returnvalue 0 1e+02 false
        (:OnSuccess
          (CallFunction|FollowPlayer)))
      (else
        (Utilities|FlowControl|Delay 1.0)
        (CallFunction|FollowPlayer)))))

(event Custom|Go%20To%20Target)

(event Custom|Run%20From%20Player
  (bind _randomlocation (Class|NavigationSystemV1|GetRandomLocationinNavigableRadius (+ (Transformation|GetActorLocation) (* (Math|Vector|Normalize (- (Transformation|GetActorLocation) (Transformation|GetActorLocation (Game|GetPlayerController 0)))) (Math|Random|RandomIntegerinRange 2000 4000))) 1e+02 0 0))
  (Variables|/Script/Engine.CharacterMovementComponent|SetMaxWalkSpeed (Variables|Character|GetCharacterMovement) 6e+02)
  (AI|AIMoveTo self _randomlocation 0 5.0 false
    (:OnSuccess
      (Variables|/Script/Engine.CharacterMovementComponent|SetMaxWalkSpeed (Variables|Character|GetCharacterMovement) 225.0)
      (CallFunction|UpdateBehaviour "NewEnumerator2"))
    (:OnFail
      (Development|PrintString "failed"))))

(event EventBeginPlay
  (CallFunction|UpdateBehaviour (Variables|Movement|GetBehaviour))
  (bind _askid_abp (Utilities|Casting|CastToKidABP (Components|SkeletalMesh|GetAnimInstance (Variables|Character|GetMesh))))
  (Variables|Default|SetAnimationBlueprint _askid_abp))

(fn ConstructionScript)

(fn UpdateBehaviour
  (params (New%20Behaviour :type NPC_Behaviour%20Enum :default "NewEnumerator1"))
  (bind _output_get (Variables|Movement|SetBehaviour New%20Behaviour))
  (switch Utilities|FlowControl|Switch|SwitchonNPC_Behaviour _output_get
    (:NewEnumerator2
      (CallFunction|FindNearbySplineforWalking)
      (CallFunction|Roam))
    (:NewEnumerator4
      (CallFunction|FollowPlayer))
    (:NewEnumerator5
      (CallFunction|RunfromPlayer))))

(fn SetCurrentGroup
  (params (Group :type Group%20Dialogue%20Object%20Reference))
  (Variables|Group|SetCurrentGroup Group))

(fn RemovefromGroup
  (Variables|Group|SetCurrentGroup 0))

(fn Lookat
  (params (LookAt :type Vector))
  (Transformation|SetActorRotation (Math|Rotator|FindRelativeLookatRotation (Transformation|GetActorTransform) LookAt)))

(fn SetActive
  (params (Enable :type Boolean))
  (Development|SetHiddeninGame (Variables|Character|GetMesh) (not Enable) false)
  (if Enable
    (bind _askid_abp (Utilities|Casting|CastToKidABP (Components|SkeletalMesh|GetAnimInstance (Variables|Character|GetMesh))))
    (Variables|Default|SetAnimationBlueprint _askid_abp)
    (Collision|SetCollisionEnabled (Variables|Collision|GetCapsuleComponent) "QueryAndPhysics")
    (Collision|SetCollisionEnabled (Variables|Default|GetNPCTalkTrigger) "QueryAndPhysics")
    (Collision|SetCollisionEnabled (Variables|Character|GetMesh) "QueryAndPhysics")
    (else
      (Collision|SetCollisionEnabled (Variables|Collision|GetCapsuleComponent) "NoCollision")
      (Collision|SetCollisionEnabled (Variables|Character|GetMesh) "NoCollision")
      (Collision|SetCollisionEnabled (Variables|Default|GetNPCTalkTrigger) "NoCollision"))))