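; TCS_GlobalFunctions is a function library of shared helpers for the Traffic Control System.
; SelectRandomRoadPath picks a random lane on a road and a random outgoing connection index from that lane.
; Two helpers compute where a value lies between two bounds, one clamped to the unit range and the other returning zero for an empty range.
; A version getter reports the system's hard-coded version and development flag.
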(fn SelectRandomRoadPath
  (params (ATC_Road :type TCS%20Road%20Path%20Object%20Reference))
  (bind _lanes (Variables|/Game/TrafficControlSystem/TCS_RoadPath.TCS_RoadPath_C|GetLanes ATC_Road))
  (bind _output_get (LocalVariables|SetSelectedLane (Math|Random|RandomIntegerinRange 0 (Utilities|Array|LastIndex _lanes))))
  (LocalVariables|SetSelectedConnection (.OutIndex (Utilities|Array|Random (.Connections (Utilities|Struct|BreakTCS_Road_Lane (Utilities|Array|Get(acopy) _lanes _output_get))))))
  (return (LocalVariables|GetSelectedLane) (LocalVariables|GetSelectedConnection)))

(fn GetPercentBetweenValuesClamped
  (params (Value :type Float%20%28double-precision%29) (Begin :type Float%20%28double-precision%29) (End :type Float%20%28double-precision%29))
  (return (Math|Float|Clamp(Float) (|((Value-Low)/(High-Low)) Value Begin End))))

(fn GetPercentBetweenValues
  (params (Value :type Float%20%28double-precision%29) (Begin :type Float%20%28double-precision%29) (End :type Float%20%28double-precision%29))
  (if (!= (- End Begin) 0.0)
    (return (|((Value-Low)/(High-Low)) Value Begin End))
    (else
      (return 0.0))))

(fn GetTCSVersion
  (return "1.1.0" false))