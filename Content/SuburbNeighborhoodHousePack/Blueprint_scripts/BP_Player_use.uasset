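; BP_Player_use is an interaction Blueprint that lets the player open and close house and garage doors.
; It enables input for player 0 on BeginPlay and reuses the IA_EnterCar action as the use trigger.
; Each press line-traces 500 units forward from the player character's camera on the Camera channel.
; The hit actor is cast to BP_Door_main and BP_Door_garage, calling OpenClose on whichever matches.
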(event `self.ReceiveBeginPlay`
  (`self.EnableInput` (`GameplayStatics.GetPlayerController` 0)))

(event `EnhancedInput|/Game/ThirdPerson/Input/Actions/IA_EnterCar`
  (params (ActionValue :type Boolean) (ElapsedSeconds :type "Float (double-precision)") (TriggeredSeconds :type "Float (double-precision)") (InputAction :type "InputAction Object Reference" :default "/Game/ThirdPerson/Input/Actions/IA_EnterCar.IA_EnterCar"))
  (bind _returnvalue (`GameplayStatics.GetPlayerCharacter` 0))
  (bind _returnvalue_2 (`self.GetComponentByClass` _returnvalue "/Script/Engine.CameraComponent"))
  (bind _returnvalue_3 (`SceneComponent.K2_GetComponentLocation` _returnvalue_2))
  (:`Started`
    (if (`KismetSystemLibrary.IsValid` _returnvalue)
      (bind _outhit (`KismetSystemLibrary.LineTraceSingle` _returnvalue_3 (+ _returnvalue_3 (* (`SceneComponent.GetForwardVector` _returnvalue_2) 500.0)) "TraceTypeQuery2" false (`|MakeArray` _returnvalue :!type "Actor Object Reference")))
      (`|ExecutionSequence`
        (:`then_0`
          (bind (_bblockinghit _binitialoverlap _time _distance _location _impactpoint _normal _impactnormal _physmat _hitactor) (`GameplayStatics.BreakHitResult` _outhit))
          (bind _asbp_door_main (cast `/Game/SuburbNeighborhoodHousePack/Blueprints/BP_Door_main` _hitactor))
          (`/Game/SuburbNeighborhoodHousePack/Blueprints/BP_Door_main.OpenClose` _asbp_door_main))
        (:`then_1`
          (bind _asbp_door_garage (cast `/Game/SuburbNeighborhoodHousePack/Blueprints/BP_door_garage` _hitactor))
          (`/Game/SuburbNeighborhoodHousePack/Blueprints/BP_door_garage.OpenClose` _asbp_door_garage))))))

(fn `UserConstructionScript`)