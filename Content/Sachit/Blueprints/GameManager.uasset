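; GameManager actor that tracks the current mission objective, showing it on the UI and marking its destination in the world.
; BeginPlay waits briefly, then creates the UI widget and cross-links it with the third-person player.
; SetObjectiveAndDestination toggles the marker and objective and moves the trigger; Tick caps the marker's distance from the player toward far targets.
; When enabled, player overlap completes the current mission's objective through a DoOnce that re-arms after a delay.
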(event `self.ReceiveBeginPlay`
  (bind _player (`self.Player`))
  (`KismetSystemLibrary.Delay` 2.0)
  (bind _returnvalue (`GameplayStatics.GetActorOfClass` "/Game/ThirdPerson/Blueprints/BP_ThirdPersonCharacter.BP_ThirdPersonCharacter_C"))
  (set `self.Player` _returnvalue)
  (bind _returnvalue_2 (`|CreateWidget` "/Game/Sachit/UI/UI.UI_C" (`GameplayStatics.GetPlayerController` 0)))
  (`UserWidget.AddToViewport` _returnvalue_2 0)
  (bind _output_get (set `self.UI` _returnvalue_2))
  (set `/Game/Sachit/UI/UI.PlayerBP` _player _output_get)
  (set `/Game/ThirdPerson/Blueprints/BP_ThirdPersonCharacter.UI` (`self.UI`) _player))

(event `self.ReceiveTick`
  (params (DeltaSeconds :type "Float (single-precision)"))
  (bind (_target_x _target_y) (`KismetMathLibrary.BreakVector` (`self.Target`)))
  (bind (_returnvalue_x _returnvalue_y) (`KismetMathLibrary.BreakVector` (`self.K2_GetActorLocation` (`self.Player`))))
  (if (`self.DestinationSet`)
    (if (> (`KismetMathLibrary.Vector_Distance` (`self.K2_GetActorLocation` (`self.Player`)) (`self.Target`)) (`self.FarAwayDistance`))
      (`SceneComponent.K2_SetWorldLocation` (`self.DestinationMarker`) (- (`self.K2_GetActorLocation` (`self.Player`)) (* (`KismetMathLibrary.Vector_Normal2D` (- (`KismetMathLibrary.MakeVector` _returnvalue_x _returnvalue_y) (`KismetMathLibrary.MakeVector` _target_x _target_y))) (`self.FarAwayDistance`))) false false)
      (else
        (`SceneComponent.K2_SetWorldLocation` (`self.DestinationMarker`) (`self.Target`) false false)))))

(event `self.MissionTrigger.OnComponentBeginOverlap`
  (params (OverlappedComponent :type "PrimitiveComponent Object Reference") (OtherActor :type "Actor Object Reference") (OtherComp :type "PrimitiveComponent Object Reference") (OtherBodyIndex :type Integer) (bFromSweep :type Boolean) (SweepResult :type "HitResult Structure (by ref)"))
  (bind _currentmission (`self.CurrentMission`))
  (if (`ActorComponent.ComponentHasTag` OtherComp "Player")
    (if (`self.PlayerOverlap`)
      (`/Engine/EditorBlueprintResources/StandardMacros.DoOnce` false :!label _label
        (:`Completed`
          (set `self.PlayerOverlap` false)
          (`/Engine/EditorBlueprintResources/StandardMacros.IsValid` _currentmission
            (:`Is Valid`
              (`/Game/Sachit/Mission/MissionBase/Mission.ObjectiveComplete` _currentmission))))))))

(event `ResetTrigger`
  (`KismetSystemLibrary.Delay` 10.0)
  (goto _label :!via `Reset`))

(fn `SetObjectiveAndDestination`
  (params (Target :type "Vector Structure") (Objective :type String) (Enable :type Boolean) (CompleteOnTriggerEnter :type Boolean))
  (bind _destinationmarker (`self.DestinationMarker`))
  (bind _ui (`self.UI`))
  (bind _completeontriggerenter (`local.CompleteOnTriggerEnter`))
  (set `self.Target` Target)
  (set `self.Objective` Objective)
  (if Enable
    (`SceneComponent.SetHiddenInGame` _destinationmarker false false)
    (`SceneComponent.SetVisibility` _destinationmarker true false)
    (set `self.DestinationSet` true)
    (`/Game/Sachit/UI/UI.SetObjective` _ui true (`self.Objective`))
    (`SceneComponent.K2_SetWorldLocation` (`self.MissionTrigger`) (`self.Target`) false false)
    (set `self.PlayerOverlap` _completeontriggerenter)
    (if _completeontriggerenter
      (`self.ResetTrigger`))
    (else
      (`SceneComponent.SetHiddenInGame` _destinationmarker false false)
      (`SceneComponent.SetVisibility` _destinationmarker false false)
      (set `self.DestinationSet` false)
      (`/Game/Sachit/UI/UI.SetObjective` _ui false "")
      (set `self.PlayerOverlap` false))))

(fn `UserConstructionScript`)