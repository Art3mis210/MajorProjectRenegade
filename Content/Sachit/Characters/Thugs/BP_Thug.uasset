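; Rifle-armed thug enemy that detects the player, aims and fires, and ragdolls on death before being destroyed after a delay.
; PawnSensing sight or noise halts it and starts a looping, delay-driven turn that aims at the player.
; Tick line-traces to the player, toggling the anim Blueprint's shoot flag or moving to the last known position.
; It also feeds the left-hand transform to the anim Blueprint.
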(event `self.ReceiveTick`
  (params (DeltaSeconds :type "Float (single-precision)"))
  ;[1 1 1] Tick
  (set `/Game/Sachit/Characters/Thugs/ABP_Thug.LeftHandTransform` (`SceneComponent.K2_GetComponentToWorld` (`self.LeftHand`)) (`self.ABP`))
  (if (`self.Alive`)
    (if (`/Game/Sachit/Characters/Thugs/ABP_Thug.PlayerFound` (`self.ABP`))
      (`self.CanThugSeePlayer`)
      (if (`self.Shooting`)
        (set `/Game/Sachit/Characters/Thugs/ABP_Thug.ShootRIfle` true (`self.ABP`))
        (else
          (set `/Game/Sachit/Characters/Thugs/ABP_Thug.ShootRIfle` false (`self.ABP`))
          (if (not (`self.MovingToLastKnownPosition`))
            (set `self.MovingToLastKnownPosition` true)
            (`|AIMoveTo` self (`self.PlayerLastKnownPosition`) null)))))))

(event `self.ReceiveBeginPlay`
  ;[1 1 1] Begin Play
  (bind _asabp_thug (cast `/Game/Sachit/Characters/Thugs/ABP_Thug` (`SkeletalMeshComponent.GetAnimInstance` (`self.Mesh`))))
  (bind _output_get (set `self.ABP` _asabp_thug))
  (set `/Game/Sachit/Characters/Thugs/ABP_Thug.LeftHandAlpha` 1.0 _output_get))

(event `self.PawnSensing.OnHearNoise`
  (params (Instigator :type "Pawn Object Reference") (Location :type "Vector Structure (by ref)") (Volume :type "Float (single-precision)"))
  (if (`self.Alive`) :!label _label
    (set `/Game/Sachit/Characters/Thugs/ABP_Thug.PlayerFound` true (`self.ABP`))
    (`|AIMoveTo` self (`self.K2_GetActorLocation`) null
      (:`then`
        (if (`self.FacingPlayer`)
          (`self.ShootAtPlayer`)
          (else
            (set `self.FacingPlayer` true)
            (`self.Face Player`)))
        (set `self.MovingToLastKnownPosition` false)))))

(event `self.PawnSensing.OnSeePawn`
  (params (Pawn :type "Pawn Object Reference"))
  (goto _label))

(event `ShootRifle`
  ;[1 1 1] Play Rifle Shoot Animation
  (`|PlayMontage` (`self.Assault_Rifle_B`) "/Game/MilitaryWeapDark/Weapons/Anims/Fire_Rifle_W_Montage.Fire_Rifle_W_Montage"))

(event `ShootAtPlayer`
  ;[1 1 1] Play Shoot Animation
  (if (`self.Alive`)
    (`self.CanThugSeePlayer`)))

(event `Face Player`
  (bind (_returnvalue_roll _returnvalue_pitch _returnvalue_yaw) (`KismetMathLibrary.BreakRotator` (`KismetMathLibrary.RInterpTo` (`self.K2_GetActorRotation`) (`KismetMathLibrary.FindLookAtRotation` (`self.K2_GetActorLocation`) (`self.K2_GetActorLocation` (`GameplayStatics.GetPlayerPawn` 0))) (`GameplayStatics.GetWorldDeltaSeconds`) 20.0)))
  ;[1 1 1] Look At Player
  (`self.K2_SetActorRotation` (`KismetMathLibrary.MakeRotator` 0.0 0.0 _returnvalue_yaw))
  (set `/Game/Sachit/Characters/Thugs/ABP_Thug.AimRotation` (`KismetMathLibrary.MakeRotator` 0.0 _returnvalue_pitch -15.0) (`self.ABP`))
  (`KismetSystemLibrary.Delay` 0.001)
  (if (`self.FacingPlayer`)
    (`self.Face Player`)))

(event `Die`
  (if (`self.Alive`)
    (set `self.Alive` false)
    (set `/Game/Sachit/Characters/Thugs/ABP_Thug.ShootRIfle` false (`self.ABP`))
    (set `/Game/Sachit/Characters/Thugs/ABP_Thug.LeftHandAlpha` 0.0 (`self.ABP`))
    (`PrimitiveComponent.SetSimulatePhysics` (`self.Mesh`) true)
    (`PrimitiveComponent.SetCollisionEnabled` (`self.CapsuleComponent`) "NoCollision")
    (`self.Killed`)
    (`self.DestroyThug`)))

(event `DestroyThug`
  (`KismetSystemLibrary.Delay` 10.0)
  (`self.K2_DestroyActor`))

(fn `CanThugSeePlayer`
  (bind (_outhit _returnvalue) (`KismetSystemLibrary.LineTraceSingleByProfile` (`self.K2_GetActorLocation`) (`self.K2_GetActorLocation` (`GameplayStatics.GetPlayerPawn` 0))))
  (if _returnvalue
    (if (`self.ActorHasTag` (`.HitActor` (`GameplayStatics.BreakHitResult` _outhit)) "Player")
      (set `self.Shooting` true)
      (set `self.PlayerLastKnownPosition` (`self.K2_GetActorLocation` (`GameplayStatics.GetPlayerPawn` 0)))
      (else
        (set `self.Shooting` false :!label _label)))
    (else
      (goto _label))))

(fn `UserConstructionScript`)