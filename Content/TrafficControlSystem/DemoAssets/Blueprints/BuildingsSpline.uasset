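; Demo-asset spline actor that scatters random building meshes along its path at construction time.
; The Construction Script steps along the spline by Spread, tracing vertically at each point and placing a mesh only where the hit actor is in AllowedHits.
; Each building sits at the hit location with random yaw and height scale.
; A separate AlignHeights function flattens all spline points to the first point's local Z.
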(fn `AlignHeights`
  (bind _spline (`self.Spline`))
  (bind (_returnvalue_x _returnvalue_y _returnvalue_z) (`KismetMathLibrary.BreakVector` (`SplineComponent.GetLocationAtSplinePoint` _spline 0 "Local")))
  (for _index (range (`SplineComponent.GetNumberOfSplinePoints` _spline))
    (bind (_returnvalue_x_2 _returnvalue_y_2) (`KismetMathLibrary.BreakVector` (`SplineComponent.GetLocationAtSplinePoint` _spline _index "Local")))
    (`SplineComponent.SetLocationAtSplinePoint` _spline _index (`KismetMathLibrary.MakeVector` _returnvalue_x_2 _returnvalue_y_2 _returnvalue_z) "Local" true)))

(fn `UserConstructionScript`
  (locals (BuildingSpread :type "Float (double-precision)" :default 0.0) (CurSplineDist :type "Float (double-precision)" :default 0.0))
  (bind _returnvalue (/ (`SplineComponent.GetSplineLength` (`self.Spline`)) (`self.Spread`)))
  (set `local.BuildingSpread` _returnvalue)
  (for _index (range (+ (`KismetMathLibrary.FFloor` _returnvalue) 1))
    (bind _returnvalue_2 (* (`self.Spread`) (`KismetMathLibrary.Conv_IntToDouble` _index)))
    (set `local.CurSplineDist` _returnvalue_2)
    (bind _returnvalue_3 (`SplineComponent.GetLocationAtDistanceAlongSpline` (`self.Spline`) _returnvalue_2 "World"))
    (bind (_outhit _returnvalue_4) (`KismetSystemLibrary.LineTraceSingle` (+ _returnvalue_3 (0.0 0.0 2000.0)) (+ _returnvalue_3 (0.0 0.0 -2000.0)) "TraceTypeQuery1"))
    (if _returnvalue_4
      (bind (_bblockinghit _binitialoverlap _time _distance _location _impactpoint _normal _impactnormal _physmat _hitactor) (`GameplayStatics.BreakHitResult` _outhit))
      (if (`KismetArrayLibrary.Array_Contains` (`self.AllowedHits`) _hitactor)
        (bind _returnvalue_5 (`AddComponent|NODE_AddStaticMeshComponent-0`))
        (`StaticMeshComponent.SetStaticMesh` _returnvalue_5 (`KismetArrayLibrary.Array_Random` (`self.Buildings`)))
        (`SceneComponent.K2_SetWorldLocationAndRotation` _returnvalue_5 _location (`KismetMathLibrary.MakeRotator` 0.0 0.0 (`KismetMathLibrary.RandomFloatInRange` 0.0 360.0)) false false)
        (`SceneComponent.SetRelativeScale3D` _returnvalue_5 (`KismetMathLibrary.MakeVector` 1.0 1.0 (`KismetMathLibrary.RandomFloatInRange` 0.7 1.3)))))))