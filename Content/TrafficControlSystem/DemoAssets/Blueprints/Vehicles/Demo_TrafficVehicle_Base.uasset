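; Base demo vehicle for the Traffic Control System, turning its traffic-vehicle events into visible driving behavior.
; Throttle, handbrake and resource-mode changes feed TCSVehiclePhysics, while steering yaws the front wheels, which reset outside driving-physics mode.
; Client initialization can randomize paint through a dynamic material with weighted common, rare or random colors, in standalone only to avoid network cost.
; An optional construction-script preview shows each wheel's travel limits as red and green mesh copies.
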(event `self.TCS_TrafficVehicle.ResourceModeChanged`
  (params (NewResourceMode :type "/Game/TrafficControlSystem/Blueprints/Vehicles/TCS_ResourceModes Enum" :default "NewEnumerator0"))
  (`/Game/TrafficControlSystem/Blueprints/Vehicles/Components/TCS_VehiclePhysics.SetDrivingPhysics` (`self.TCS_VehiclePhysics`) (`|EnumEquality` NewResourceMode "NewEnumerator2"))
  (`self.ResetSteering` NewResourceMode))

(event `self.TCS_TrafficVehicle.UpdateThrottle`
  (params (NewThrottle :type "Float (double-precision)"))
  (`/Game/TrafficControlSystem/Blueprints/Vehicles/Components/TCS_VehiclePhysics.SetThrottle` (`self.TCS_VehiclePhysics`) NewThrottle))

(event `self.TCS_TrafficVehicle.UpdateHandbrake`
  (params (NewHandbrake :type Boolean))
  (`/Game/TrafficControlSystem/Blueprints/Vehicles/Components/TCS_VehiclePhysics.SetHandbrake` (`self.TCS_VehiclePhysics`) NewHandbrake))

(event `self.TCS_TrafficVehicle.UpdateSteering`
  (params (NewSteering :type "Float (double-precision)"))
  (`SceneComponent.K2_SetRelativeRotation` (`self.Wheel_Front_Driver`) (`KismetMathLibrary.MakeRotator` 0.0 0.0 (* NewSteering (`self.MaxSteeringAngle`))) false false)
  (`SceneComponent.K2_SetRelativeRotation` (`self.Wheel_Front_Passenger`) (`KismetMathLibrary.MakeRotator` 0.0 0.0 (* NewSteering (`self.MaxSteeringAngle`))) false false))

(event `ResetSteering`
  (params (Mode :type "/Game/TrafficControlSystem/Blueprints/Vehicles/TCS_ResourceModes Enum" :default "NewEnumerator0"))
  (if (`|EnumInequality` Mode "NewEnumerator2")
    (`SceneComponent.K2_SetRelativeRotation` (`self.Wheel_Front_Passenger`) (`KismetMathLibrary.MakeRotator` 0.0) false false)
    (`SceneComponent.K2_SetRelativeRotation` (`self.Wheel_Front_Driver`) (`KismetMathLibrary.MakeRotator` 0.0) false false)))

(event `self.TCS_TrafficVehicle.ClientInitialized`
  ;[1 1 1] Singleplayer Only -- Networking this would add a network cost unrelated to
  ; the main asset. So I have decided this leave this out for multiplayer, as it would pollute any network testing of the asset
  (if (`self.RandomizePaints`)
    (`self.RandomizePaint`)))

(fn `CreateWheelTravelPreview`
  (locals (ChildrenCache :type "Array of SceneComponent Object Reference") (Wheels :type "Array of /Game/TrafficControlSystem/Blueprints/Vehicles/Components/TCS_Vehicle_Wheel Object Reference"))
  (bind _output_get (set `local.ChildrenCache` (`SceneComponent.GetChildrenComponents` (`self.VehicleMesh`) true)))
  (for _array_element _output_get
    (bind _astcs_vehicle_wheel (cast `/Game/TrafficControlSystem/Blueprints/Vehicles/Components/TCS_Vehicle_Wheel` _array_element))
    (`KismetArrayLibrary.Array_Add` (`local.Wheels`) _astcs_vehicle_wheel))
  (for _array_element_2 (`local.Wheels`)
    (bind _asstatic_mesh_component (cast `StaticMeshComponent` (`SceneComponent.GetChildComponent` _array_element_2 0)))
    (bind _returnvalue (`AddComponent|NODE_AddStaticMeshComponent-0` :`bManualAttachment` true :`RelativeTransform` (`KismetMathLibrary.MakeTransform` (`KismetMathLibrary.MakeVector` 0.0 0.0 (`/Game/TrafficControlSystem/Blueprints/Vehicles/Components/TCS_Vehicle_Wheel.TravelUp` _array_element_2)))))
    (bind _staticmesh (`StaticMeshComponent.StaticMesh` _asstatic_mesh_component))
    (`StaticMeshComponent.SetStaticMesh` _returnvalue _staticmesh)
    (`SceneComponent.K2_AttachToComponent` _returnvalue _array_element_2 "None" "KeepRelative" "KeepRelative" "KeepRelative" true)
    (`self.SetMeshMaterial` _returnvalue "/Game/TrafficControlSystem/Materials/Debug/Debug_Halo_Red.Debug_Halo_Red")
    (bind _returnvalue_2 (`AddComponent|NODE_AddStaticMeshComponent-1` :`bManualAttachment` true :`RelativeTransform` (`KismetMathLibrary.MakeTransform` (`KismetMathLibrary.MakeVector` 0.0 0.0 (* (`/Game/TrafficControlSystem/Blueprints/Vehicles/Components/TCS_Vehicle_Wheel.TravelDown` _array_element_2) -1.0)))))
    (`StaticMeshComponent.SetStaticMesh` _returnvalue_2 _staticmesh)
    (`SceneComponent.K2_AttachToComponent` _returnvalue_2 _array_element_2 "None" "KeepRelative" "KeepRelative" "KeepRelative" true)
    (`self.SetMeshMaterial` _returnvalue_2 "/Game/TrafficControlSystem/Materials/Debug/Debug_Halo_Green.Debug_Halo_Green")))

(fn `RandomizePaint`
  (returns (ChangedPaint :type Boolean) (NewMaterial :type "MaterialInstanceDynamic Object Reference"))
  (bind _vehiclemesh (`self.VehicleMesh`))
  (bind _returnvalue (`MeshComponent.GetMaterialIndex` _vehiclemesh "Paint1"))
  (if (`KismetSystemLibrary.IsStandalone`)
    (if (>= _returnvalue 0)
      (bind _returnvalue_2 (`PrimitiveComponent.CreateDynamicMaterialInstance` _vehiclemesh _returnvalue "/Game/TrafficControlSystem/DemoAssets/Materials/AutomotivePaint/Demo_CarPaint_DarkTeal.Demo_CarPaint_DarkTeal" "None"))
      (`MaterialInstanceDynamic.SetVectorParameterValue` _returnvalue_2 "Color" (select `bool` (`KismetMathLibrary.RandomBoolWithWeight` 0.95) :`false` (make `LinearColor` (`KismetMathLibrary.RandomFloat`) (`KismetMathLibrary.RandomFloat`) (`KismetMathLibrary.RandomFloat`) 1.0) :`true` (select `bool` (`KismetMathLibrary.RandomBoolWithWeight` 0.9) :`false` (`KismetArrayLibrary.Array_Random` (`self.PaintColorsRare`)) :`true` (`KismetArrayLibrary.Array_Random` (`self.PaintColors`)))))
      (return true _returnvalue_2)
      (else
        (return false null)))))

(fn `SetMeshMaterial`
  (params (Mesh :type "StaticMeshComponent Object Reference") (Material :type "MaterialInterface Object Reference"))
  (for _index (range (+ (`PrimitiveComponent.GetNumMaterials` Mesh) 1))
    (`PrimitiveComponent.SetMaterial` Mesh _index Material)))

(fn `UserConstructionScript`
  (if (`self.PreviewWheelTravel`)
    (`self.CreateWheelTravelPreview`)))